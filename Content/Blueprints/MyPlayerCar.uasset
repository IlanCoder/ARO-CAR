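; MyPlayerCar is the player-controlled car Blueprint, with driving, power-up firing, crash response and checkpoint tracking.
; Its event graph only forwards events: input axes and the FirePowerUp action call matching functions defined outside this file, and Hit passes its normal to AfterCrashVelocity.
; Overlapping an actor whose class casts to CheckPoint passes that actor's location and rotation to SetCheckpoint.
; BeginPlay, Tick and the construction script are empty.
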(event EventBeginPlay)

(event EventTick
  (params (DeltaSeconds :type Float%20%28single-precision%29)))

(event Collision|EventHit
  (params (MyComp :type Primitive%20Component%20Object%20Reference) (Other :type Actor%20Object%20Reference) (OtherComp :type Primitive%20Component%20Object%20Reference) (bSelfMoved :type Boolean) (HitLocation :type Vector :default "0, 0, 0") (HitNormal :type Vector :default "0, 0, 0") (NormalImpulse :type Vector :default "0, 0, 0") (Hit :type Hit%20Result%20Structure%20%28by%20ref%29))
  (Class|PlayerCar|AfterCrashVelocity HitNormal))

(event Collision|EventActorBeginOverlap
  (params (OtherActor :type Actor%20Object%20Reference))
  (Utilities|Casting|CastToCheckPointClass (Utilities|GetClass OtherActor))
  (Class|PlayerCar|SetCheckpoint (Transformation|GetActorLocation OtherActor) (Transformation|GetActorRotation OtherActor)))

(event Input|ActionEvents|InputActionFirePowerUp
  (params (Key :type Key%20Structure))
  ;[1 1 1] Input
  (:Pressed
    (Class|PlayerCar|SpawnPowerUp)))

(event Input|AxisEvents|InputAxisBreak
  (params (AxisValue :type Float%20%28single-precision%29))
  ;[1 1 1] Input
  (Class|PlayerCar|CarBreak AxisValue))

(event Input|AxisEvents|InputAxisUp
  (params (AxisValue :type Float%20%28single-precision%29))
  ;[1 1 1] Input
  (Class|PlayerCar|Up AxisValue))

(event Input|AxisEvents|InputAxisAccelerate
  (params (AxisValue :type Float%20%28single-precision%29))
  ;[1 1 1] Input
  (Class|PlayerCar|Accelerate AxisValue))

(event Input|AxisEvents|InputAxisRotate
  (params (AxisValue :type Float%20%28single-precision%29))
  ;[1 1 1] Input
  (Class|PlayerCar|Rotate AxisValue))

(event Input|AxisEvents|InputAxisRight
  (params (AxisValue :type Float%20%28single-precision%29))
  ;[1 1 1] Input
  (Class|PlayerCar|Right AxisValue))

(fn ConstructionScript)